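; Interaction component that lets the player interact with actors implementing BPI_Interaction.
; On BeginPlay it creates WB_Interact_Message, then a looping timer runs CapsuleTrace, a short sphere sweep along the owner's forward vector, to set TargetActor.
; IA_Interact calls InteractWithMessage on that target with the player character.
; CapsuleTrace calls LookAtMessage but always blanks the widget; the unused SphereTrace variant displays the returned text.
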(event Custom|BeginInteraction
  (Utilities|Time|SetTimerbyEvent (delegate Custom|UpdateInteraction) 0.2 true))

(event Custom|UpdateInteraction
  (CallFunction|CapsuleTrace))

(event Input|EnhancedActionEvents|EnhancedInputActionIA_Interact
  (params (ActionValue :type Boolean) (ElapsedSeconds :type Float%20%28double-precision%29) (TriggeredSeconds :type Float%20%28double-precision%29) (InputAction :type Input%20Action%20Object%20Reference :default "/Game/ThirdPerson/Input/Actions/IA_Interact.IA_Interact"))
  (:Started
    (bind _target_actor (Variables|Default|GetTarget%20Actor)
      (:then
        (Class|BPIInteraction|Interactwith(Message) _target_actor (CallFunction|GetPlayerCharacter)))
      (:else))))

(event EventBeginPlay
  (CallFunction|CreateInteractMessage)
  (CallFunction|BeginInteraction))

(fn CreateInteractMessage
  (bind _returnvalue (UserInterface|CreateWidget "/Game/Interakcja/WB_Interact_Message.WB_Interact_Message_C"))
  (bind _output_get (Variables|Default|SetWB_Interact_Message _returnvalue))
  (UserInterface|Viewport|AddtoViewport _output_get 0))

(fn SphereTrace
  (bind _returnvalue (Components|GetOwner))
  (bind _returnvalue_2 (Transformation|GetActorLocation _returnvalue))
  (bind (_outhit _returnvalue_3) (Collision|SphereTraceByChannel _returnvalue_2 _returnvalue_2 1.5e+02 "TraceTypeQuery3" false 0 "ForOneFrame"))
  (if _returnvalue_3
    (if (Utilities|DoesObjectImplementInterface (.HitActor (Collision|BreakHitResult _outhit)) "/Game/Interakcja/BPI_Interaction.BPI_Interaction_C")
      (bind _output_get (Variables|Default|SetTarget%20Actor (.HitActor (Collision|BreakHitResult _outhit))))
      (bind _message (Class|BPIInteraction|Lookat(Message) _output_get))
      (Default|SetMessage (Variables|Default|GetWB_Interact_Message) _message)
      (else
        (Variables|Default|SetTarget%20Actor 0)
        (Default|SetMessage (Variables|Default|GetWB_Interact_Message))))
    (else
      (Variables|Default|SetTarget%20Actor 0)
      (Default|SetMessage (Variables|Default|GetWB_Interact_Message)))))

(fn CapsuleTrace
  (bind _returnvalue (Components|GetOwner))
  (bind _returnvalue_2 (Transformation|GetActorLocation _returnvalue))
  (bind (_outhit _returnvalue_3) (Collision|SphereTraceByChannel _returnvalue_2 (+ _returnvalue_2 (* (Transformation|GetActorForwardVector _returnvalue) 1.5e+02)) 2e+01 "TraceTypeQuery3" false 0 "ForOneFrame"))
  (if _returnvalue_3
    (if (Utilities|DoesObjectImplementInterface (.HitActor (Collision|BreakHitResult _outhit)) "/Game/Interakcja/BPI_Interaction.BPI_Interaction_C")
      (bind _output_get (Variables|Default|SetTarget%20Actor (.HitActor (Collision|BreakHitResult _outhit))))
      (Class|BPIInteraction|Lookat(Message) _output_get)
      (Default|SetMessage (Variables|Default|GetWB_Interact_Message))
      (else
        (Variables|Default|SetTarget%20Actor 0)
        (Default|SetMessage (Variables|Default|GetWB_Interact_Message))))
    (else
      (Variables|Default|SetTarget%20Actor 0)
      (Default|SetMessage (Variables|Default|GetWB_Interact_Message)))))